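; BP_Enemy_Static is an enemy Blueprint that keeps turning to face the player character while it is alive.
; After the parent BeginPlay, a looping timer fires LookPlayer every 0.05 seconds instead of using Tick.
; LookPlayer applies only the yaw of a look-at rotation toward player 0 and does nothing once IsDead is set.
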(event Custom|LookPlayer
  (if (not (Variables|Default|GetIsDead))
    (Transformation|SetActorRotation (Math|Rotator|MakeRotator 0.0 0.0 (.yaw (Math|Rotator|FindLookatRotation (Transformation|GetActorLocation) (Transformation|GetActorLocation (Game|GetPlayerCharacter 0))))))))

(event EventBeginPlay
  (|CallParentFunction)
  (Utilities|Time|SetTimerbyEvent (delegate Custom|LookPlayer) 0.05 true true))

(fn ConstructionScript
  (|CallParentFunction))