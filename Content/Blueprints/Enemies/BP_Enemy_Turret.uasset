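; Enemy turret that turns to face the player and fires projectiles at them.
; PawnSensing starts a self-repeating, cooldown-gated attack and a looping timer updates yaw, until the player exits a lose-sight sphere.
; Damage is rate-limited and routed by component tag: shield hits are ignored, while weak point hits deal boosted damage and can destroy it.
; At zero HP it enables mesh physics and disables capsule, shield and weak point.
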(event OnComponentEndOverlap(PlayerLooseSightSphere)
  (params (OverlappedComponent :type Primitive%20Component%20Object%20Reference) (OtherActor :type Actor%20Object%20Reference) (OtherComp :type Primitive%20Component%20Object%20Reference) (OtherBodyIndex :type Integer))
  (if (Variables|Default|GetPlayerInSight)
    (Variables|Default|SetPlayerInSight false)))

(event OnSeePawn(PawnSensing)
  (params (Pawn :type Pawn%20Object%20Reference))
  (Variables|Default|SetPlayerInSight true)
  (CallFunction|AttackPlayer))

(event Custom|AttackPlayer
  (if (and (Variables|Default|GetPlayerInSight) (not (Variables|Default|GetIsDead)))
    (if (Variables|Default|GetCanAttack)
      (Variables|Default|SetCanAttack false)
      (Game|SpawnActorfromClass "/Game/Blueprints/Enemies/BP_EnemyProjectile.BP_EnemyProjectile_C" (Math|Transform|MakeTransform (Transformation|GetWorldLocation (Variables|Default|GetShootPoint)) (Math|Rotator|FindLookatRotation (Transformation|GetActorLocation) (Transformation|GetActorLocation (Game|GetPlayerCharacter 0))) "1.000000,1.000000,1.000000") "AdjustIfPossibleButAlwaysSpawn" "MultiplyWithRoot" 0 (Variables|Default|GetAttackDamage) 0)
      (Utilities|FlowControl|Delay (Variables|Default|GetAttackCooldown))
      (Variables|Default|SetCanAttack true)
      (CallFunction|AttackPlayer)
      (else
        (Utilities|FlowControl|Delay 0.2)
        (CallFunction|AttackPlayer)))))

(event Custom|LookPlayer
  (if (and (Variables|Default|GetPlayerInSight) (not (Variables|Default|GetIsDead)))
    (Transformation|SetActorRotation (Math|Rotator|MakeRotator 0.0 0.0 (.yaw (Math|Rotator|FindLookatRotation (Transformation|GetActorLocation) (Transformation|GetActorLocation (Game|GetPlayerCharacter 0))))))))

(event EventBeginPlay
  (|CallParentFunction)
  (Utilities|Time|SetTimerbyEvent (delegate Custom|LookPlayer) 0.05 true true))

(event EventDeath
  (bind _shield (Variables|Default|GetShield))
  (bind _weakpoint (Variables|Default|GetWeakPoint))
  (if (not (Variables|Default|GetIsDead))
    (Variables|Default|SetIsDead true)
    (Physics|SetSimulatePhysics (Variables|Character|GetMesh) true)
    (Collision|SetCollisionEnabled (Variables|Default|GetCapsuleComponent) "NoCollision")
    (Rendering|SetVisibility _weakpoint false true)
    (Collision|SetCollisionEnabled _weakpoint "NoCollision")
    (Rendering|SetVisibility _shield false true)
    (Collision|SetCollisionEnabled _shield "NoCollision")))

(event EventDamageObject
  (params (Damage :type Integer) (DamageBoosted :type Integer) (DamageSource :type Actor%20Object%20Reference) (HitComponent :type Actor%20Component%20Object%20Reference))
  (if (<= (Variables|Default|GetCurrentDamageCooldown) 0.0)
    (Variables|Default|SetCurrentDamageCooldown (Variables|Default|GetMaxDamageCooldown))
    (Utilities|IsValid HitComponent
      (:Is%20Valid
        (if (not (Components|ComponentHasTag HitComponent "Shield"))
          (if (Components|ComponentHasTag HitComponent "WeakPoint")
            (bind _result (Math|Integer|DecrementInt (Variables|Default|GetWeakPointHitResist))
              (:%20%20
                (if (<= _result 0)
                  (CallFunction|DestroyWeakPoint))
                (Utilities|ApplyDamage DamageBoosted)))
            (else
              (Utilities|ApplyDamage Damage :!label _label)))))
      (:Is%20Not%20Valid
        (goto _label)))))

(fn ConstructionScript
  (|CallParentFunction))