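; Shielded melee enemy that chases the player and deals damage through an attack zone.
; Pawn sensing and a looping line-trace timer gate a self-repeating AIMoveTo chase, with attacks limited by a reset timer.
; Component tags route incoming hits: Shield blocks with sparks and sound, WeakPoint kills instantly, and others reduce HP, with a damage cooldown on non-shield component hits.
; Death ragdolls the mesh and disables the capsule, shield and weak point.
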(event OnSeePawn(PawnSensing)
  (params (Pawn :type Pawn%20Object%20Reference))
  (Utilities|IsValid (Utilities|Array|Get(acopy) (Collision|GetOverlappingActors "/Game/Blueprints/BP_Player.BP_Player_C" :!class /Script/Engine.Actor))
    (:Is%20Valid
      (Variables|Default|SetPlayerInRange true)
      (CallFunction|FollowPlayer))
    (:Is%20Not%20Valid
      (Variables|Default|SetPlayerInRange false))))

(event OnComponentEndOverlap(PlayerLooseSightSphere)
  (params (OverlappedComponent :type Primitive%20Component%20Object%20Reference) (OtherActor :type Actor%20Object%20Reference) (OtherComp :type Primitive%20Component%20Object%20Reference) (OtherBodyIndex :type Integer))
  (if (Variables|Default|GetPlayerInSight)
    (Variables|Default|SetPlayerInSight false)
    (AI|AIMoveTo self (Transformation|GetActorLocation (Game|GetPlayerCharacter 0)) 0 25.0 false)))

(event Custom|FollowPlayer
  (bind _attackzone (Variables|Default|GetAttackZone))
  (if (and (Variables|Default|GetCanChase) (not (Variables|Default|GetIsDead)))
    (AI|AIMoveTo self "0, 0, 0" (Game|GetPlayerCharacter 0) 5e+01 false
      (:OnSuccess
        (if (Variables|Default|GetCanAttack)
          (Variables|Default|SetCanAttack false)
          (Transformation|SetActorRotation (Math|Rotator|MakeRotator 0.0 0.0 (.yaw (Math|Rotator|FindLookatRotation (Transformation|GetActorLocation) (Transformation|GetActorLocation (Game|GetPlayerCharacter 0))))))
          (bind (_outactors _returnvalue) (Collision|ComponentOverlapActors _attackzone (Transformation|GetWorldTransform _attackzone) (Utilities|Array|MakeArray "ObjectTypeQuery3") "/Game/Blueprints/BP_Player.BP_Player_C"))
          (if _returnvalue
            (for _array_element _outactors
              (Class|BPIDamageable|DamageObject(Message) _array_element (Variables|Default|GetAttackDamage) 0 self 0 "" "0, 0, 0")
              (Utilities|Time|SetTimerbyEvent (delegate Custom|ResetAttack) 3.0 true true)
              (Utilities|FlowControl|Delay 1.0)
              (CallFunction|FollowPlayer))
            (else
              (Utilities|Time|SetTimerbyEvent (delegate Custom|ResetAttack) 3.0 true true)
              (Utilities|FlowControl|Delay 1.0)
              (CallFunction|FollowPlayer)))
          (else
            (CallFunction|FollowPlayer))))
      (:OnFail
        (CallFunction|FollowPlayer)))))

(event Custom|ResetAttack
  (Variables|Default|SetCanAttack true))

(event Custom|CheckPlayerSight
  (bind _returnvalue (Transformation|GetActorLocation))
  (if (and (Variables|Default|GetPlayerInRange) (not (Variables|Default|GetIsDead)))
    (bind _outhit (Collision|LineTraceByChannel _returnvalue (+ _returnvalue (* (Math|Vector|GetForwardVector (Math|Rotator|FindLookatRotation (Transformation|GetActorLocation) (Transformation|GetActorLocation (Game|Player|GetPlayerPawn 0)))) 5e+03)) "TraceTypeQuery1" false 0 "None"))
    (Variables|Default|SetPlayerInSight (Class|GameplayStatics|ObjectIsA (.HitActor (Collision|BreakHitResult _outhit)) "/Game/Blueprints/BP_Player.BP_Player_C"))))

(event EventBeginPlay
  (|CallParentFunction)
  (Utilities|Time|SetTimerbyEvent (delegate Custom|CheckPlayerSight) 0.5 true true))

(event EventTick
  (params (DeltaSeconds :type Float%20%28single-precision%29))
  (|CallParentFunction DeltaSeconds)
  (Variables|Default|SetCanChase (and (Variables|Default|GetPlayerInRange) (Variables|Default|GetPlayerInSight))))

(event EventDeath
  (bind _shield (Variables|Default|GetShield))
  (bind _weakpoint (Variables|Default|GetWeakPoint))
  (if (not (Variables|Default|GetIsDead))
    (Variables|Default|SetIsDead true)
    (Physics|SetSimulatePhysics (Variables|Character|GetMesh) true)
    (Collision|SetCollisionEnabled (Variables|Default|GetCapsuleComponent) "NoCollision")
    (Rendering|SetVisibility _weakpoint false true)
    (Collision|SetCollisionEnabled _weakpoint "NoCollision")
    (Rendering|SetVisibility _shield false true)
    (Collision|SetCollisionEnabled _shield "NoCollision")))

(event EventDamageObject
  (params (Damage :type Integer) (DamageBoosted :type Integer) (DamageSource :type Actor%20Object%20Reference) (HitComponent :type Actor%20Component%20Object%20Reference) (CustomParam :type String) (HitLocation :type Vector :default "0, 0, 0"))
  (bind _weakpoint (Variables|Default|GetWeakPoint))
  (bind _returnvalue (Transformation|GetWorldRotation _weakpoint))
  (Utilities|IsValid HitComponent
    (:Is%20Valid
      (if (Components|ComponentHasTag HitComponent "Shield")
        (Niagara|SpawnSystematLocation "/Game/Tech_VFX/Bart/VFX/NS_Spark_Shield_01.NS_Spark_Shield_01" HitLocation)
        (Audio|PlaySound2D "/Game/Sound/SFX/HitEnemiesShieldGLOW.HitEnemiesShieldGLOW" 1.0 1.0 0.0 0 0)
        (elif (<= (Variables|Default|GetCurrentDamageCooldown) 0.0)
          (Variables|Default|SetCurrentDamageCooldown (Variables|Default|GetMaxDamageCooldown))
          (if (Components|ComponentHasTag HitComponent "WeakPoint")
            (Audio|PlaySound2D "/Game/Sound/SFX/HitWeakSpotEnemies.HitWeakSpotEnemies" 1.0 1.0 0.0 0 0)
            (Niagara|SpawnSystematLocation "/Game/Tech_VFX/Melon/vfx/NS_hit_point_faible_02.NS_hit_point_faible_02" (Transformation|GetWorldLocation _weakpoint) (Math|Rotator|MakeRotator (+ (.roll _returnvalue) 9e+01) (.pitch _returnvalue) (+ (.yaw _returnvalue) 9e+01)))
            (CallFunction|Death)
            (else
              (Niagara|SpawnSystematLocation "/Game/Tech_VFX/Melon/vfx/NS_hit_enemy_01.NS_hit_enemy_01" "0, 0, 0" :!label _label)
              (Utilities|ApplyDamage Damage))))))
    (:Is%20Not%20Valid
      (goto _label))))

(fn ConstructionScript
  (|CallParentFunction))