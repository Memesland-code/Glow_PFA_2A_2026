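; BP_EnemyMain is an enemy Blueprint that manages health, damage intake, a destructible weak point and death.
; DamageObject ignores hits during a cooldown counted down in Tick, applying boosted damage when the hit component is tagged WeakPoint.
; Each weak-point hit lowers its resistance until it is hidden and loses collision.
; ApplyDamage triggers a one-time Death at zero health, which ragdolls the mesh and disables capsule and weak-point collision.
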(event Custom|Death
  (bind _weakpoint (Variables|Default|GetWeakPoint))
  (if (not (Variables|Stats|GetIsDead))
    (Variables|Stats|SetIsDead true)
    (Physics|SetSimulatePhysics (Variables|Character|GetMesh) true)
    (Collision|SetCollisionEnabled (Variables|Collision|GetCapsuleComponent) "NoCollision")
    (Collision|SetCollisionEnabled _weakpoint "NoCollision")
    (Rendering|SetVisibility _weakpoint false true)))

(event Custom|DestroyWeakPoint
  (bind _weakpoint (Variables|Default|GetWeakPoint))
  (Rendering|SetVisibility _weakpoint false true)
  (Collision|SetCollisionEnabled _weakpoint "NoCollision"))

(event EventBeginPlay
  (Variables|Stats|SetCurrentHP (Variables|Stats|GetMaxHP)))

(event EventTick
  (params (DeltaSeconds :type Float%20%28single-precision%29))
  (if (> (Variables|Stats|GetCurrentDamageCooldown) 0.0)
    (Variables|Stats|SetCurrentDamageCooldown (- (Variables|Stats|GetCurrentDamageCooldown) DeltaSeconds))))

(event EventDamageObject
  (params (Damage :type Integer) (DamageBoosted :type Integer) (DamageSource :type Actor%20Object%20Reference) (HitComponent :type Actor%20Component%20Object%20Reference) (CustomParam :type String))
  (if (<= (Variables|Stats|GetCurrentDamageCooldown) 0.0)
    (Variables|Stats|SetCurrentDamageCooldown (Variables|Stats|GetMaxDamageCooldown))
    (Utilities|IsValid HitComponent
      (:Is%20Valid
        (if (Components|ComponentHasTag HitComponent "WeakPoint")
          (bind _result (Math|Integer|DecrementInt (Variables|WeakPoint|GetWeakPointHitResist))
            (:%20%20
              (if (<= _result 0)
                (CallFunction|DestroyWeakPoint))
              (Utilities|ApplyDamage DamageBoosted)))
          (else
            (Utilities|ApplyDamage Damage :!label _label))))
      (:Is%20Not%20Valid
        (goto _label)))))

(fn ConstructionScript)