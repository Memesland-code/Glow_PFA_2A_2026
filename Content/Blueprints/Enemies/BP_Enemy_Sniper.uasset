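; Sniper enemy that turns to face the player and fires projectiles from its shoot point, extending a parent enemy class.
; Pawn sensing plus an overlap check sets the in-range flag, cleared when the player exits the lose-sight sphere.
; A timed visibility trace confirms line of sight; both flags together gate timer-driven yaw tracking and the self-recalling attack loop, paced by a cooldown.
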(event OnComponentEndOverlap(PlayerLooseSightSphere)
  (params (OverlappedComponent :type Primitive%20Component%20Object%20Reference) (OtherActor :type Actor%20Object%20Reference) (OtherComp :type Primitive%20Component%20Object%20Reference) (OtherBodyIndex :type Integer))
  (if (and (Variables|Default|GetPlayerInRange) (Class|GameplayStatics|ObjectIsA OtherActor "/Game/Blueprints/BP_Player.BP_Player_C"))
    (Variables|Default|SetPlayerInRange false)))

(event OnSeePawn(PawnSensing)
  (params (Pawn :type Pawn%20Object%20Reference))
  (Utilities|IsValid (Utilities|Array|Get(acopy) (Collision|GetOverlappingActors "/Game/Blueprints/BP_Player.BP_Player_C" :!class /Script/Engine.Actor))
    (:Is%20Valid
      (Variables|Default|SetPlayerInRange true)
      (CallFunction|AttackPlayer))
    (:Is%20Not%20Valid
      (Variables|Default|SetPlayerInRange false))))

(event Custom|AttackPlayer
  (if (and (Variables|Default|GetCanChase) (not (Variables|Default|GetIsDead)))
    (if (Variables|Default|GetCanAttack)
      (Variables|Default|SetCanAttack false)
      (Game|SpawnActorfromClass "/Game/Blueprints/Enemies/BP_EnemyProjectile.BP_EnemyProjectile_C" (Math|Transform|MakeTransform (Transformation|GetWorldLocation (Variables|Default|GetShootPoint)) (Math|Rotator|FindLookatRotation (Transformation|GetActorLocation) (Transformation|GetActorLocation (Game|GetPlayerCharacter 0))) "1.000000,1.000000,1.000000") "AdjustIfPossibleButAlwaysSpawn" "MultiplyWithRoot" 0 (Variables|Default|GetAttackDamage) 0)
      (Utilities|FlowControl|Delay (Variables|Default|GetAttackCooldown))
      (Variables|Default|SetCanAttack true)
      (CallFunction|AttackPlayer)
      (Audio|PlaySound2D "/Game/Sound/SFX/ShootEnemiesGLOW.ShootEnemiesGLOW" 1.0 1.0 0.0 0 0)
      (else
        (Utilities|FlowControl|Delay 0.2)
        (CallFunction|AttackPlayer)))))

(event Custom|CheckPlayerSight
  (bind _returnvalue (Transformation|GetActorLocation))
  (if (Variables|Default|GetPlayerInRange)
    (bind _outhit (Collision|LineTraceByChannel _returnvalue (+ _returnvalue (* (Math|Vector|GetForwardVector (Math|Rotator|FindLookatRotation (Transformation|GetActorLocation) (Transformation|GetActorLocation (Game|Player|GetPlayerPawn 0)))) 5e+03)) "TraceTypeQuery1" false 0 "None"))
    (Variables|Default|SetPlayerInSight (Class|GameplayStatics|ObjectIsA (.HitActor (Collision|BreakHitResult _outhit)) "/Game/Blueprints/BP_Player.BP_Player_C"))))

(event Custom|LookPlayer
  (if (and (Variables|Default|GetCanChase) (not (Variables|Default|GetIsDead)))
    (Transformation|SetActorRotation (Math|Rotator|MakeRotator 0.0 0.0 (.yaw (Math|Rotator|FindLookatRotation (Transformation|GetActorLocation) (Transformation|GetActorLocation (Game|GetPlayerCharacter 0))))))))

(event EventBeginPlay
  (|CallParentFunction)
  (Utilities|Time|SetTimerbyEvent (delegate Custom|LookPlayer) 0.05 true true)
  (Utilities|Time|SetTimerbyEvent (delegate Custom|CheckPlayerSight) 0.5 true true))

(event EventTick
  (params (DeltaSeconds :type Float%20%28single-precision%29))
  (|CallParentFunction DeltaSeconds)
  (Variables|Default|SetCanChase (and (Variables|Default|GetPlayerInRange) (Variables|Default|GetPlayerInSight))))

(fn ConstructionScript
  (|CallParentFunction))