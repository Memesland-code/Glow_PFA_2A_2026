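; BP_Enemy_Rusher is a melee enemy that chases the player on sight and attacks up close.
; PawnSensing starts a FollowPlayer loop using AIMoveTo, which re-runs itself after each arrival.
; On arrival, if off cooldown, it faces the player, damages BP_Player actors overlapping AttackZone, and starts a looping ResetAttack timer.
; An end overlap on PlayerLooseSightSphere drops sight and sends it to the player's current location.
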(event OnSeePawn(PawnSensing)
  (params (Pawn :type Pawn%20Object%20Reference))
  (Variables|Default|SetPlayerInSight true)
  (CallFunction|FollowPlayer))

(event OnComponentEndOverlap(PlayerLooseSightSphere)
  (params (OverlappedComponent :type Primitive%20Component%20Object%20Reference) (OtherActor :type Actor%20Object%20Reference) (OtherComp :type Primitive%20Component%20Object%20Reference) (OtherBodyIndex :type Integer))
  (if (Variables|Default|GetPlayerInSight)
    (Variables|Default|SetPlayerInSight false)
    (AI|AIMoveTo self (Transformation|GetActorLocation (Game|GetPlayerCharacter 0)) 0 25.0 false)))

(event Custom|FollowPlayer
  (bind _attackzone (Variables|Default|GetAttackZone))
  (if (Variables|Default|GetPlayerInSight)
    (AI|AIMoveTo self "0, 0, 0" (Game|GetPlayerCharacter 0) 5e+01 false
      (:OnSuccess
        (if (Variables|Default|GetCanAttack)
          (Variables|Default|SetCanAttack false)
          (Transformation|SetActorRotation (Math|Rotator|MakeRotator 0.0 0.0 (.yaw (Math|Rotator|FindLookatRotation (Transformation|GetActorLocation) (Transformation|GetActorLocation (Game|GetPlayerCharacter 0))))))
          (bind (_outactors _returnvalue) (Collision|ComponentOverlapActors _attackzone (Transformation|GetWorldTransform _attackzone) (Utilities|Array|MakeArray "ObjectTypeQuery3") "/Game/Blueprints/BP_Player.BP_Player_C"))
          (if _returnvalue
            (for _array_element _outactors
              (Class|BPIDamageable|ApplyDamage(Message) _array_element (Variables|Default|GetAttackDamage) self)
              (Utilities|Time|SetTimerbyEvent (delegate Custom|ResetAttack) 3.0 true true)
              (Utilities|FlowControl|Delay 1.0)
              (CallFunction|FollowPlayer))
            (else
              (Utilities|Time|SetTimerbyEvent (delegate Custom|ResetAttack) 3.0 true true)
              (Utilities|FlowControl|Delay 1.0)
              (CallFunction|FollowPlayer)))
          (else
            (CallFunction|FollowPlayer)))))))

(event Custom|ResetAttack
  (Variables|Default|SetCanAttack true))

(event EventBeginPlay
  (|CallParentFunction) ; This node is disabled and will not be called.\nDrag off pins to build functionality.
)

(fn ConstructionScript
  (|CallParentFunction))