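; Boss enemy character that jumps around and out of the arena, attacks with carried or thrown cars, and blocks arena points with cars as phases progress.
; AIC_Boss starts the fight, and actions report completion through event calls while blackboard states track phases.
; Front weak point hits open the back door, and each back hit costs a life until death shows the win screen.
; Stun hits, beam slowdown and a chase timer also steer behavior.
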(event Custom|Death
  (bind _backweakpoint (Variables|Default|GetBackWeakpoint))
  (bind _weakpoint (Variables|Default|GetWeakPoint))
  (bind _caractor (Variables|CarLaunch|GetCarActor))
  (bind _frontweakpoint (Variables|Default|GetFrontWeakPoint))
  ;[0.15 0 0 0.5] Damage and death
  (if (not (Variables|Default|GetIsDead))
    (Variables|Default|SetIsDead true)
    (if (Utilities|IsValid _caractor)
      (Actor|DestroyActor _caractor))
    (Niagara|SpawnSystematLocation "/Game/Tech_VFX/elodia/NS_vfx/NS_explosion_boss.NS_explosion_boss" (Transformation|GetWorldLocation (Variables|Default|GetFrontWeakPoint)))
    (Collision|SetCollisionEnabled (Variables|Default|GetCapsuleComponent) "NoCollision")
    (Collision|SetCollisionEnabled _weakpoint "NoCollision")
    (Rendering|SetVisibility _weakpoint false true)
    (Collision|SetCollisionEnabled _backweakpoint "NoCollision")
    (Rendering|SetVisibility _backweakpoint false true)
    (Collision|SetCollisionEnabled _frontweakpoint "NoCollision")
    (Rendering|SetVisibility _frontweakpoint false true)
    (Collision|SetCollisionResponsetoChannel (Variables|Default|GetSK_Boss) "ECC_Camera" "ECR_Ignore")
    (Animation|Montage|PlayMontage (Variables|Character|GetMesh) "/Game/Animations/Anims_Retargeted/Anim_boss_death1_Montage.Anim_boss_death1_Montage"
      (:OnBlendOut
        (Physics|SetSimulatePhysics (Variables|Default|GetSK_Boss) true)
        (Utilities|FlowControl|Delay 5.0)
        (bind _returnvalue (UserInterface|CreateWidget "/Game/Blueprints/UI/WBP_Win.WBP_Win_C"))
        (UserInterface|Viewport|AddtoViewport _returnvalue 0)))))

(event Custom|JumpOnLocation
  (params (ShouldRemoveAnyCar :type Boolean) (ShouldAOE :type Boolean))
  (bind _playerloosesightsphere (Variables|Default|GetPlayerLooseSightSphere))
  (bind _overlappingactors (Collision|GetOverlappingActors _playerloosesightsphere "/Game/Blueprints/BP_Player.BP_Player_C" :!class /Script/Engine.PrimitiveComponent))
  (bind _output (Utilities|Array|Get(acopy) _overlappingactors))
  (if (and ShouldRemoveAnyCar (Utilities|IsValid (Variables|CarLaunch|GetCarActor)))
    (CallFunction|ThrowCar)
    (Utilities|FlowControl|Delay 0.5))
  (Utilities|FlowControl|Sequence
    (:then_0
      (Utilities|Array|Clear (Variables|HighJump|GetUsedPoints))
      (switch Utilities|FlowControl|Switch|SwitchonE_BossStates (Utilities|Enum|ByteToEnumE_BossStates (Class|BlackboardComponent|GetValueasEnum (Variables|AI|GetBlackboardRef) (Utilities|Name|MakeLiteralName "States")))
        (:NewEnumerator5
          (Variables|HighJump|SetUsedPoints (Variables|HighJump|GetInArenaPoints) :!label _label))
        (:NewEnumerator2
          (Variables|HighJump|SetUsedPoints (Variables|HighJump|GetArenaBorderPoints)))
        (:NewEnumerator3
          (Variables|HighJump|SetUsedPoints (Variables|HighJump|GetOutArenaPoints)))
        (:NewEnumerator4
          (goto _label))))
    (:then_1
      (bind _output_get (Variables|HighJump|SetSelectedJumpPoint (Transformation|GetActorLocation (Utilities|Array|Get(acopy) (Variables|HighJump|GetUsedPoints) (Math|Random|RandomInteger (Utilities|Array|Length (Variables|HighJump|GetUsedPoints)))))))
      (Transformation|SetActorRotation (Math|Rotator|MakeRotator 0.0 0.0 (.yaw (Math|Rotator|FindLookatRotation (Transformation|GetActorLocation) _output_get))))
      (bind _output_get_2 (Variables|HighJump|SetStartLocation (Transformation|GetActorLocation)))
      (Variables|HighJump|SetJumpMaxHeight (+ (.Z (Math|Vector|BreakVector _output_get_2)) 1.5e+03))
      (Animation|Montage|PlayMontage (Variables|Character|GetMesh) "/Game/Animations/Anims_Retargeted/Anim_Bosscarjump1_Montage.Anim_Bosscarjump1_Montage"
        (:then
          (bind (_direction _alpha _z_alpha) (Timeline|JumpingTimeline PlayFromStart)
            (:Update
              (if (<= _alpha 0.5)
                (Transformation|SetActorLocation (Math|Vector|MakeVector (.x (Math|Vector|Lerp(Vector) (Math|Vector|MakeVector (.x (Variables|HighJump|GetStartLocation)) (.y (Variables|HighJump|GetStartLocation)) 0.0) (Math|Vector|MakeVector (.x (Variables|HighJump|GetSelectedJumpPoint)) (.y (Variables|HighJump|GetSelectedJumpPoint)) 0.0) _alpha)) (.y (Math|Vector|Lerp(Vector) (Math|Vector|MakeVector (.x (Variables|HighJump|GetStartLocation)) (.y (Variables|HighJump|GetStartLocation)) 0.0) (Math|Vector|MakeVector (.x (Variables|HighJump|GetSelectedJumpPoint)) (.y (Variables|HighJump|GetSelectedJumpPoint)) 0.0) _alpha)) (Math|Float|Lerp (.z (Variables|HighJump|GetStartLocation)) (Variables|HighJump|GetJumpMaxHeight) _z_alpha)) false false)
                (else
                  (Transformation|SetActorLocation (Math|Vector|MakeVector (.x (Math|Vector|Lerp(Vector) (Math|Vector|MakeVector (.x (Variables|HighJump|GetStartLocation)) (.y (Variables|HighJump|GetStartLocation)) 0.0) (Math|Vector|MakeVector (.x (Variables|HighJump|GetSelectedJumpPoint)) (.y (Variables|HighJump|GetSelectedJumpPoint)) 0.0) _alpha)) (.y (Math|Vector|Lerp(Vector) (Math|Vector|MakeVector (.x (Variables|HighJump|GetStartLocation)) (.y (Variables|HighJump|GetStartLocation)) 0.0) (Math|Vector|MakeVector (.x (Variables|HighJump|GetSelectedJumpPoint)) (.y (Variables|HighJump|GetSelectedJumpPoint)) 0.0) _alpha)) (Math|Float|Lerp (.z (Variables|HighJump|GetSelectedJumpPoint)) (Variables|HighJump|GetJumpMaxHeight) _z_alpha)) false false))))
            (:Finished
              (if ShouldAOE
                (Development|PrintString "BP_Boss Warning: JumpOnLocation: No AOE feedback")
                (Utilities|IsValid _output
                  (:Is%20Valid
                    (Class|BPIDamageable|DamageObject(Message) _output (Variables|AttackDamages|GetAOE_AttackDamage) 0 self))
                  (:Is%20Not%20Valid
                    _)))
              (Default|CallOnJumpingEnd))))))))

(event Custom|ArenaCarAnim
  (params (RepeatTimes :type Integer) (IsStart :type Boolean))
  (bind _returnvalue (Game|SpawnActorfromClass "/Game/Blueprints/Enemies/BOSS/BP_Car.BP_Car_C" (Math|Transform|MakeTransform (Transformation|GetWorldLocation (Variables|Default|GetCarLaunchPoint)) (Math|Rotator|FindLookatRotation (Transformation|GetWorldLocation (Variables|Default|GetCarLaunchPoint)) (Transformation|GetActorLocation (Game|Player|GetPlayerPawn 0))) "1.000000,1.000000,1.000000") "Undefined" "MultiplyWithRoot" 0 true 0))
  (Variables|CarLaunch|SetCarLaunchedLocation (Transformation|GetWorldLocation (Variables|Default|GetCarLaunchPoint)))
  (if IsStart
    (Variables|CarLaunch|SetChosenArenaBlockPoint (Variables|CarLaunch|GetArenaEntryBlockPoint))
    (else
      (bind _output_get (Variables|CarLaunch|SetChosenArenaBlockPoint (Utilities|Array|Get(acopy) (Variables|CarLaunch|GetArenaBlockingPoints) (Math|Random|RandomIntegerinRange 0 (- (Utilities|Array|Length (Variables|CarLaunch|GetArenaBlockingPoints)) 1)))))
      (Utilities|Array|RemoveItem (Variables|CarLaunch|GetArenaBlockingPoints) _output_get)))
  (bind _output_get_2 (Variables|CarLaunch|SetCarLaunchDestination (Transformation|GetActorLocation (Variables|CarLaunch|GetChosenArenaBlockPoint))))
  (Variables|CarLaunch|SetCarLaunchZ_Rotation (.yaw (Math|Rotator|FindLookatRotation (Transformation|GetActorLocation) _output_get_2)))
  (bind _alpha (Timeline|Timeline PlayFromStart)
    (:Update
      (Transformation|SetActorLocationAndRotation _returnvalue (Math|Vector|Lerp(Vector) (Variables|CarLaunch|GetCarLaunchedLocation) (Math|Vector|MakeVector (.x (Variables|CarLaunch|GetCarLaunchDestination)) (.y (Variables|CarLaunch|GetCarLaunchDestination)) (+ (.z (Variables|CarLaunch|GetCarLaunchDestination)) 1.3e+02)) _alpha) (Math|Rotator|MakeRotator (.roll (Transformation|GetWorldRotation (Variables|/Game/Blueprints/Enemies/BOSS/BP_Car.BP_Car_C|GetCar _returnvalue))) (Math|Float|Lerp 0.0 -9e+01 _alpha) (Variables|CarLaunch|GetCarLaunchZ_Rotation))))
    (:Finished
      (if (> RepeatTimes 0)
        (Utilities|FlowControl|Delay 2.0)
        (CallFunction|ArenaCarAnim (- RepeatTimes 1) false)
        (else
          (Default|CallOnArenaCarPlaced))))))

(event Custom|BackDoorControl
  (params (RotationValue :type Float%20%28double-precision%29))
  (Variables|WeakPoint|SetCurrentBackDoorOpen (.roll (Variables|/Script/Engine.SceneComponent|GetRelativeRotation (Variables|Default|GetBackDoor))))
  (bind _alpha (Timeline|BackDoorRotation PlayFromStart)
    (:Update
      (Transformation|SetRelativeRotation (Variables|Default|GetBackDoor) (Math|Rotator|MakeRotator (Math|Float|Lerp (Variables|WeakPoint|GetCurrentBackDoorOpen) RotationValue _alpha) 0.0 0.0) false false))))

(event Custom|FlinchEffect
  (params (IsBackHit :type Boolean))
  ;[0.15 0 0 0.5] Damage and death
  (if IsBackHit
    (Variables|WeakPoint|SetMaterialRestaurationTime 5.0)
    (else
      (Variables|WeakPoint|SetMaterialRestaurationTime 0.2)))
  (Rendering|Material|SetMaterial (Variables|Default|GetSK_Boss) 1 (Variables|WeakPoint|GetWeakpointFlinchMat))
  (Rendering|Material|SetMaterial (Variables|Default|GetSK_Boss) 3 (Variables|WeakPoint|GetWeakpointFlinchMat))
  (Utilities|FlowControl|Delay (Variables|WeakPoint|GetMaterialRestaurationTime))
  (Rendering|Material|SetMaterial (Variables|Default|GetSK_Boss) 1 (Variables|WeakPoint|GetWeakpointBaseMat))
  (Rendering|Material|SetMaterial (Variables|Default|GetSK_Boss) 3 (Variables|WeakPoint|GetWeakpointBaseMat)))

(event Custom|StartBoss
  (Variables|AI|SetHasStarted true)
  (bind _asaic_boss (Utilities|Casting|CastToAIC_Boss (AI|GetAIController self)))
  (Default|StartBoss _asaic_boss))

(event Custom|Attack
  (bind _randomchasetime (Variables|AI|GetRandomChaseTime))
  (Variables|AI|SetCurrentChaseTime (Math|Random|RandomFloatinRange (.x _randomchasetime) (.y _randomchasetime)))
  (Development|PrintString "BP_Boss Warning: Basic attack animation not set")
  (Utilities|FlowControl|Delay 1.0)
  (Class|BPIDamageable|DamageObject(Message) (Utilities|Array|Get(acopy) (Collision|GetOverlappingActors (Variables|Default|GetBasicAttackZone) "/Game/Blueprints/BP_Player.BP_Player_C" :!class /Script/Engine.PrimitiveComponent)) (Variables|AttackDamages|GetBasicAttackDamage) 0 self)
  (Utilities|FlowControl|Delay 1.0)
  (Default|CallOnAttackEnd))

(event Custom|GetCar
  (bind _returnvalue (Game|SpawnActorfromClass "/Game/Blueprints/Enemies/BOSS/BP_Car.BP_Car_C" (Math|Transform|MakeTransform "0, 0, 0" "90.000000,90.000000,0.000000" "1.000000,1.000000,1.000000") "Undefined" "MultiplyWithRoot" 0 false 0))
  (bind _output_get (Variables|CarLaunch|SetCarActor _returnvalue))
  (Collision|SetActorEnableCollision _output_get false)
  (bind _returnvalue_2 (Transformation|AttachComponentToComponent _output_get (Variables|Default|GetSK_Boss) "CarCarry" "SnapToTarget" "KeepRelative" "KeepWorld" true))
  (if (not _returnvalue_2)
    (Development|PrintString "BP_Boss Error: Attach car to boss did not worked. Check boss' attachment socket" true true "(R=1.000000,G=0.000000,B=0.000000,A=1.000000)" 3e+01)))

(event Custom|RegisterWPState
  (Variables|Intern|SetRegisteredCanFrontWP (Variables|WeakPoint|GetCanFrontBeHit))
  (Variables|Intern|SetRegisteredBackFrontWP (Variables|WeakPoint|GetCanBackBeHit)))

(event Custom|ApplyRegisteredWPState
  (Variables|WeakPoint|SetCanFrontBeHit (Variables|Intern|GetRegisteredCanFrontWP))
  (Variables|WeakPoint|SetCanBackBeHit (Variables|Intern|GetRegisteredBackFrontWP)))

(event Custom|StartCarRushingTimer
  (bind _carrushingtime (Variables|AI|GetCarRushingTime))
  (Utilities|FlowControl|Delay 0.0)
  (Variables|AI|SetRandomMeleeCar (Math|Random|RandomBool))
  (AI|Components|Blackboard|SetValueasBool (Variables|AI|GetBlackboardRef) (Utilities|Name|MakeLiteralName "MeleeWithCar") (Variables|AI|GetRandomMeleeCar))
  (if (Variables|AI|GetRandomMeleeCar)
    (Variables|AI|SetCurrentCarRushingTime (Math|Random|RandomFloatinRange (.x _carrushingtime) (.y _carrushingtime)))
    (Variables|AI|SetIsRushing true)
    (Animation|Montage|PlayMontage (Variables|Character|GetMesh) "/Game/Animations/Anims_Retargeted/Anim_walkboss_withcar1_Montage.Anim_walkboss_withcar1_Montage"
      (:then
        _)))
  (Default|CallOnCarRushChecked))

(event Custom|MeleeCarAttack
  (Animation|Montage|PlayMontage (Variables|Character|GetMesh) "/Game/Animations/Anims_Retargeted/Anim_Boss_hitwithcar1_Montage.Anim_Boss_hitwithcar1_Montage"
    (:then
      (Utilities|FlowControl|Delay 1.0)
      (Class|BPIDamageable|DamageObject(Message) (Utilities|Array|Get(acopy) (Collision|GetOverlappingActors (Variables|Default|GetMeleeCarAttackZone) "/Game/Blueprints/BP_Player.BP_Player_C" :!class /Script/Engine.PrimitiveComponent)) (Variables|AttackDamages|GetBasicAttackDamage) 0 self)
      (bind _caractor (Variables|CarLaunch|GetCarActor)
        (:then
          (Development|PrintString "BP_Boss Warning: Make car destroy on hit ground")
          (Actor|DestroyActor _caractor)
          (Utilities|FlowControl|Delay 1.0)
          (Default|CallMeleeCarAttackEnd))
        (:else
          (Development|PrintString "BP_Boss Error: MeleeCarAttack: CarActor is not valid"))))))

(event Custom|ThrowCar
  (bind _returnvalue (Game|GetPlayerCharacter 0))
  (bind _returnvalue_2 (Transformation|GetActorLocation))
  (bind _caractor (Variables|CarLaunch|GetCarActor))
  (bind _returnvalue_3 (Transformation|GetActorLocation _returnvalue))
  (Utilities|IsValid _caractor
    (:Is%20Valid
      (Actor|DestroyActor _caractor))
    (:Is%20Not%20Valid
      _))
  (Animation|Montage|PlayMontage (Variables|Character|GetMesh) "/Game/Animations/Anims_Retargeted/Anim_Boss_hitwithcar1_Montage.Anim_Boss_hitwithcar1_Montage"
    (:then
      (bind _returnvalue_4 (Game|SpawnActorfromClass "/Game/Blueprints/Enemies/BOSS/BP_Car.BP_Car_C" (Math|Transform|MakeTransform (Transformation|GetWorldLocation (Variables|Default|GetCarLaunchPoint)) (Math|Rotator|FindLookatRotation (Transformation|GetWorldLocation (Variables|Default|GetCarLaunchPoint)) (Transformation|GetActorLocation (Game|Player|GetPlayerPawn 0))) "1.000000,1.000000,1.000000") "Undefined" "MultiplyWithRoot" 0 false 0))
      (Physics|SetSimulatePhysics (Variables|/Game/Blueprints/Enemies/BOSS/BP_Car.BP_Car_C|GetCar _returnvalue_4) true)
      (Physics|AddImpulse (Variables|/Game/Blueprints/Enemies/BOSS/BP_Car.BP_Car_C|GetCar _returnvalue_4) (* (Math|Vector|GetForwardVector (Math|Rotator|FindLookatRotation _returnvalue_2 _returnvalue_3)) (Math|Vector|Distance(Vector) _returnvalue_2 _returnvalue_3)) "None" true)
      (Utilities|FlowControl|Delay 0.0)
      (Default|CallOnCarLaunched))))

(event Custom|PlaceArenaCar
  (params (IsStart :type Boolean))
  (bind _caractor (Variables|CarLaunch|GetCarActor))
  (Utilities|IsValid _caractor
    (:Is%20Valid
      (Actor|DestroyActor _caractor))
    (:Is%20Not%20Valid
      _))
  (if IsStart
    (CallFunction|ArenaCarAnim 0 true)
    (else
      (switch int (Variables|Stats|GetCurrentLifeBar)
        (:Default
          (Development|PrintString "BP_Boss Error: PlaceArenaCar: Boss life logic to place car in arena is not valid!" true true "(R=1.000000,G=0.000000,B=0.000000,A=1.000000)" 3e+01))
        (:1
          (CallFunction|ArenaCarAnim 1 false))
        (:2
          (CallFunction|ArenaCarAnim 0 false))))))

(event EventBeginPlay
  (bind _randomchasetime (Variables|AI|GetRandomChaseTime))
  (Variables|Stats|SetCurrentLifeBar (Variables|Stats|GetMaxLifeBar))
  (Variables|WeakPoint|SetCanFrontBeHit true)
  (Variables|Intern|SetUnusedArenaBlockingPoints (Variables|CarLaunch|GetArenaBlockingPoints))
  (Variables|AI|SetCurrentChaseTime (Math|Random|RandomFloatinRange (.x _randomchasetime) (.y _randomchasetime)))
  (Variables|WeakPoint|SetWeakpointBaseMat (Utilities|Array|Get(acopy) (Rendering|Material|GetMaterials (Variables|Default|GetSK_Boss)) 1))
  (CallFunction|GetCar)
  (Utilities|FlowControl|Sequence
    (:then_0
      (if (not (Components|ComponentHasTag (Variables|Default|GetFrontWeakPoint) "FrontWeakPoint"))
        (Development|PrintText "BP_BOSS Error: Front weak point has not a valid check tag FrontWeakPoint" true true "(R=1.000000,G=0.001000,B=0.000000,A=1.000000)" 3e+01)))
    (:then_1
      (if (not (Components|ComponentHasTag (Variables|Default|GetBackWeakpoint) "BackWeakPoint"))
        (Development|PrintText "BP_BOSS Error: Back weak point has not a valid check tag BackWeakPoint" true true "(R=1.000000,G=0.001000,B=0.000000,A=1.000000)" 3e+01)))
    (:then_2
      (if (Utilities|Array|IsEmpty (Variables|HighJump|GetOutArenaPoints))
        (Development|PrintText "BP_BOSS Error: JumpOutPoints Array is empty. Should have at least 1 value" true true "(R=1.000000,G=0.001000,B=0.000000,A=1.000000)" 3e+01)))
    (:then_3
      (Utilities|IsValid (Variables|CarLaunch|GetArenaEntryBlockPoint)
        (:Is%20Not%20Valid
          (Development|PrintText "BP_BOSS Error: ArenaEntryBlockPoint variable is empty. Should have at least 1 value" true true "(R=1.000000,G=0.001000,B=0.000000,A=1.000000)" 3e+01))))))

(event EventTick
  (params (DeltaSeconds :type Float%20%28single-precision%29))
  (bind _randomchasetime (Variables|AI|GetRandomChaseTime))
  (Utilities|FlowControl|Sequence
    (:then_0
      (if (Variables|AI|GetIsRushing)
        (bind _output_get (Variables|AI|SetCurrentCarRushingTime (- (Variables|AI|GetCurrentCarRushingTime) DeltaSeconds)))
        (if (<= _output_get 0.0)
          (Variables|AI|SetIsRushing false)
          (AI|Components|Blackboard|SetValueasBool (Variables|AI|GetBlackboardRef) (Utilities|Name|MakeLiteralName "MeleeWithCar") false))))
    (:then_1
      (if (> (Variables|Default|GetCurrentDamageCooldown) 0.0)
        (Variables|Default|SetCurrentDamageCooldown (- (Variables|Default|GetCurrentDamageCooldown) DeltaSeconds))))
    (:then_2
      (bind _output_get_2 (Variables|Stats|SetRecoverSpeedOnUltCooldown (- (Variables|Stats|GetRecoverSpeedOnUltCooldown) DeltaSeconds)))
      (if (<= _output_get_2 0.0)
        (Variables|/Script/Engine.CharacterMovementComponent|SetMaxWalkSpeed (Variables|Character|GetCharacterMovement) 4e+02)))
    (:then_3
      (Utilities|IsValid (Variables|AI|GetBlackboardRef)
        (:Is%20Valid
          (if (Math|Boolean|ANDBoolean (Utilities|Enum|Equal(Enum) (Utilities|Enum|ByteToEnumE_BossStates (Class|BlackboardComponent|GetValueasEnum (Variables|AI|GetBlackboardRef) (Utilities|Name|MakeLiteralName "States"))) "NewEnumerator0") (not (ScalableFloat|GetValueasBool (Variables|AI|GetBlackboardRef) (Utilities|Name|MakeLiteralName "HasCar"))) (not (Variables|WeakPoint|GetCanBackBeHit)))
            (bind _output_get_3 (Variables|AI|SetCurrentChaseTime (- (Variables|AI|GetCurrentChaseTime) DeltaSeconds)))
            (if (<= _output_get_3 0.0)
              (AI|Components|Blackboard|SetValueasEnum (Variables|AI|GetBlackboardRef) (Utilities|Name|MakeLiteralName "States") (Utilities|Enum|LiteralenumE_BossStates "NewEnumerator3")))
            (else
              (Variables|AI|SetCurrentChaseTime (Math|Random|RandomFloatinRange (.x _randomchasetime) (.y _randomchasetime))))))))))

(event EventDamageObject
  (params (Damage :type Integer) (DamageBoosted :type Integer) (DamageSource :type Actor%20Object%20Reference) (HitComponent :type Actor%20Component%20Object%20Reference) (CustomParam :type String))
  ;[0.15 0 0 0.5] Damage and death
  (if (Variables|AI|GetHasStarted)
    (Utilities|FlowControl|Sequence
      (:then_0
        (Utilities|IsValid HitComponent
          (:Is%20Valid
            (if (Components|ComponentHasTag HitComponent "FrontWeakPoint")
              (if (Variables|WeakPoint|GetCanFrontBeHit) :!label _label
                (CallFunction|FlinchEffect false)
                (bind _returnvalue (Niagara|SpawnSystematLocation "/Game/Tech_VFX/Melon/vfx/NS_hit_point_faible_01.NS_hit_point_faible_01" (Transformation|GetWorldLocation (Variables|Default|GetFrontWeakPoint))))
                (Utilities|FlowControl|Sequence
                  (:then_0
                    (bind _result (Math|Integer|IncrementInt (Variables|WeakPoint|GetFrontHitCount))
                      (:%20%20
                        (if (>= _result (Variables|WeakPoint|GetFrontHitResistance))
                          (Variables|WeakPoint|SetFrontHitCount 0)
                          (Variables|WeakPoint|SetCanFrontBeHit false)
                          (Variables|WeakPoint|SetCanBackBeHit true)
                          (CallFunction|BackDoorControl (Variables|WeakPoint|GetBackDoorOpenedValue))
                          (if (not (ScalableFloat|GetValueasBool (AI|GetBlackboard 0) (Utilities|Name|MakeLiteralName "HasCar")))
                            (AI|Components|Blackboard|SetValueasEnum (AI|GetBlackboard 0) (Utilities|Name|MakeLiteralName "States") (Utilities|Enum|LiteralenumE_BossStates "NewEnumerator6")))))))
                  (:then_1
                    (Utilities|FlowControl|Delay 1.0)
                    (Components|DestroyComponent _returnvalue))))))))
      (:then_1
        (Utilities|IsValid HitComponent
          (:Is%20Valid
            (if (Components|ComponentHasTag HitComponent "BackWeakPoint")
              (if (Variables|WeakPoint|GetCanBackBeHit) :!label _label_2
                (Variables|WeakPoint|SetCanBackBeHit false)
                (Variables|WeakPoint|SetCanFrontBeHit true)
                (bind _result_2 (Math|Integer|DecrementInt (Variables|Stats|GetCurrentLifeBar))
                  (:%20%20
                    (if (<= _result_2 0)
                      (CallFunction|Death)
                      (else
                        (CallFunction|FlinchEffect true)
                        (Niagara|SpawnSystematLocation "/Game/Tech_VFX/Melon/vfx/NS_hit_point_faible_01.NS_hit_point_faible_01" (Transformation|GetWorldLocation (Variables|Default|GetBackWeakpoint)))
                        (CallFunction|BackDoorControl (Variables|WeakPoint|GetBackDoorClosedValue))
                        (AI|Components|Blackboard|SetValueasEnum (AI|GetBlackboard 0) (Utilities|Name|MakeLiteralName "States") (Utilities|Enum|LiteralenumE_BossStates "NewEnumerator2")))))))))))
      (:then_2
        (bind _result_3 (Math|Integer|IncrementInt (Variables|Stats|GetStunCurrentHit))
          (:%20%20
            (if (and (>= _result_3 (Variables|Stats|GetStunMaxHit)) (Utilities|Enum|Equal(Enum) (Utilities|Enum|ByteToEnumE_BossStates (Class|BlackboardComponent|GetValueasEnum (AI|GetBlackboard 0) (Utilities|Name|MakeLiteralName "States"))) "NewEnumerator0"))
              (AI|Components|Blackboard|SetValueasEnum (AI|GetBlackboard 0) (Utilities|Name|MakeLiteralName "States") (Utilities|Enum|LiteralenumE_BossStates "NewEnumerator6"))
              (Variables|Stats|SetStunCurrentHit 0)))))
      (:then_3
        (if (Utilities|Enum|Equal(Enum) CustomParam "BEAM")
          (Variables|/Script/Engine.CharacterMovementComponent|SetMaxWalkSpeed (Variables|Character|GetCharacterMovement) 25.0)
          (if (<= (Variables|Default|GetCurrentDamageCooldown) 0.0)
            (Variables|Default|SetCurrentDamageCooldown (Variables|Default|GetMaxDamageCooldown))
            (Variables|Stats|SetRecoverSpeedOnUltCooldown 2.0)
            (Utilities|FlowControl|Sequence
              (:then_0
                (goto _label))
              (:then_1
                (goto _label_2)))))))))

(fn ConstructionScript)