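; Interactable energy recharge station that notifies the player it was used and plays a camera and VFX sequence.
; On Interact, a timeline lerps the player's camera boom arm length and spawns a recharge effect at the station, destroyed after a delay.
; DoOnce gates block restarts and repeat spawns until the timeline finishes, which resets them and fires the OnRechargeFinished dispatcher.
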(event EventInteract
  (params (Interactor :type Actor%20Object%20Reference))
  (bind _asbp_player (Utilities|Casting|CastToBP_Player Interactor))
  (Default|UsedRechargePoint _asbp_player self)
  (bind _output_get (Variables|Default|SetAs%20BP%20Player _asbp_player))
  (Components|Activation|Activate (Variables|/Game/Blueprints/BP_Player.BP_Player_C|GetCameraBoom _output_get) false)
  (Utilities|FlowControl|DoOnce false :!label _label
    (:Completed
      (bind _aim_zoom (Timeline|Timeline PlayFromStart)
        (:Update
          (Variables|/Script/Engine.SpringArmComponent|SetTargetArmLength (Variables|/Game/Blueprints/BP_Player.BP_Player_C|GetCameraBoom _output_get) (Math|Float|Lerp 3e+02 4e+02 _aim_zoom))
          (Utilities|FlowControl|DoOnce false :!label _label_2
            (:Completed
              (bind _returnvalue (Game|SpawnActorfromClass "/Game/Blueprints/Energy/BP_recharge_vfx_01.BP_recharge_vfx_01_C" (Math|Transform|MakeTransform (Transformation|GetActorLocation) "0, 0, 0" "1.000000,1.000000,1.000000") "Undefined" "MultiplyWithRoot" 0 0))
              (Utilities|FlowControl|Delay 5.0)
              (Actor|DestroyActor _returnvalue))))
        (:Finished
          (Utilities|FlowControl|Sequence
            (:then_0
              (goto _label_2 Reset))
            (:then_1
              (goto _label Reset))
            (:then_2
              (Default|CallOnRechargeFinished))))))))

(fn ConstructionScript)