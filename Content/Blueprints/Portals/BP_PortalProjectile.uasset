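; BP_PortalProjectile is a projectile that places a linked pair of in and out portals when it hits something.
; Whoever spawns it registers a portal reference plus precomputed positions and rotations for both portals, which it stores.
; On component hit it passes those stored values to PlacePortals on that reference, ignoring the actual impact point, then destroys itself.
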(event OnComponentHit(PortalProjectile)
  (params (HitComponent :type Primitive%20Component%20Object%20Reference) (OtherActor :type Actor%20Object%20Reference) (OtherComp :type Primitive%20Component%20Object%20Reference) (NormalImpulse :type Vector :default "0, 0, 0") (Hit :type Hit%20Result%20Structure%20%28by%20ref%29))
  (Default|PlacePortals (Variables|Default|GetPortalRef) (Variables|Default|GetOutPortalPosition) (Variables|Default|GetOutPortalRotation) (Variables|Default|GetInPortalPosition) (Variables|Default|GetInPortalRotation))
  (Actor|DestroyActor))

(event Custom|RegisterPortalPlacement
  (params (PortalRef :type BP%20Portal%20Object%20Reference) (OutPortalPosition :type Vector) (OutPortalRotation :type Rotator) (InPortalPosition :type Vector) (InPortalRotation :type Rotator))
  (Variables|Default|SetPortalRef PortalRef)
  (Variables|Default|SetOutPortalPosition OutPortalPosition)
  (Variables|Default|SetOutPortalRotation OutPortalRotation)
  (Variables|Default|SetInPortalPosition InPortalPosition)
  (Variables|Default|SetInPortalRotation InPortalRotation))

(fn ConstructionScript)