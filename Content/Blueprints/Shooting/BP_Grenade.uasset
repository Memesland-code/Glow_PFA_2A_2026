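; BP_Grenade is a timed physics grenade that explodes after a cooldown, damages enemies within its explosion radius, then destroys itself.
; Overlapping components are reduced to one damage entry per BP_EnemyMain in a map, with WeakPoint-tagged components doubling base damage and AvoidDamageCheck ones skipped.
; Each registered enemy then receives a damage message.
; PassPortal teleports the grenade, remaps its velocity from entry to exit portal space and ignores one collision channel afterward.
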(event Custom|Explode
  (Utilities|Map|Clear (Variables|Default|GetRegisterDamages))
  (for _array_element (Class|PrimitiveComponent|GetOverlappingComponents (Variables|Default|GetExplosionRadius))
    (if (not (Components|ComponentHasTag _array_element "AvoidDamageCheck"))
      (if (Components|ComponentHasTag _array_element "WeakPoint")
        (Variables|Default|SetDamageToApply (* (Variables|Default|GetBaseDamage) 2))
        (else
          (Variables|Default|SetDamageToApply (Variables|Default|GetBaseDamage))))
      (if (Class|GameplayStatics|ObjectIsA (Components|GetOwner _array_element) "/Game/Blueprints/Enemies/BP_EnemyMain.BP_EnemyMain_C")
        (bind _asbp_enemy_main (Utilities|Casting|CastToBP_EnemyMain (Components|GetOwner _array_element)))
        (if (.ReturnValue (Utilities|Map|Find (Variables|Default|GetRegisterDamages) _asbp_enemy_main))
          (if (> (Variables|Default|GetDamageToApply) 0)
            (Utilities|Map|Add (Variables|Default|GetRegisterDamages) _asbp_enemy_main (Utilities|Struct|MakeF_GrenadeDamage (.hitcomponent (.Value (Utilities|Map|Find (Variables|Default|GetRegisterDamages) _asbp_enemy_main))) (Variables|Default|GetDamageToApply))))
          (else
            (Utilities|Map|Add (Variables|Default|GetRegisterDamages) _asbp_enemy_main (Utilities|Struct|MakeF_GrenadeDamage (.hitcomponent (.Value (Utilities|Map|Find (Variables|Default|GetRegisterDamages) _asbp_enemy_main))) (Variables|Default|GetDamageToApply))))))))
  (bind _keys (Utilities|Map|Keys (Variables|Default|GetRegisterDamages)))
  (for _array_element_2 _keys
    (if (not (Class|GameplayStatics|ObjectIsA _array_element_2 "/Game/Blueprints/BP_Player.BP_Player_C"))
      (Class|BPIDamageable|DamageObject(Message) _array_element_2 (.damage (.Value (Utilities|Map|Find (Variables|Default|GetRegisterDamages) _array_element_2))) (.damage (.Value (Utilities|Map|Find (Variables|Default|GetRegisterDamages) _array_element_2))) self (.hitcomponent (.Value (Utilities|Map|Find (Variables|Default|GetRegisterDamages) _array_element_2))))))
  (Actor|DestroyActor))

(event EventPassPortal
  (params (TargetLocation :type Vector :default "0, 0, 0") (TargetRotation :type Rotator :default "0, 0, 0") (EntryPortal :type Transform) (ExitPortal :type Transform))
  (bind _returnvalue (Physics|GetPhysicsLinearVelocity (Variables|Default|GetGrenade) "None"))
  (Transformation|SetActorLocationAndRotation TargetLocation TargetRotation)
  (Physics|SetPhysicsLinearVelocity (Variables|Default|GetGrenade) (Math|Transform|TransformDirection ExitPortal (Math|Transform|InverseTransformDirection EntryPortal _returnvalue)) false "None")
  (Collision|SetCollisionResponsetoChannel (Variables|Default|GetGrenade) "ECC_GameTraceChannel3" "ECR_Ignore"))

(event EventBeginPlay
  (Utilities|FlowControl|Delay (Variables|Default|GetExplosionCooldown))
  (CallFunction|Explode))

(fn ConstructionScript)