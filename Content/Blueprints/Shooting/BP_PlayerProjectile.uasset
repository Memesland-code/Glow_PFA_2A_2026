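; BP_PlayerProjectile is the player's shot, which damages what it hits and can travel through portals.
; On hit, it passes base and weak-point damage plus the hit component to non-player BPI_Damageable actors, triggers the player's hit feedback, then destroys itself.
; PassPortal teleports it, redirects its velocity along the new forward vector at the same speed, and ignores GameTraceChannel3 from then on.
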(event EventPassPortal
  (params (TargetLocation :type Vector :default "0, 0, 0") (TargetRotation :type Rotator :default "0, 0, 0"))
  (Variables|Default|SetPassVelocity (Math|Vector|VectorLength (Variables|/Script/Engine.MovementComponent|GetVelocity (Variables|Default|GetProjectileMovement))))
  (Transformation|SetActorLocationAndRotation TargetLocation TargetRotation)
  (Variables|/Script/Engine.MovementComponent|SetVelocity (Variables|Default|GetProjectileMovement) (* (Transformation|GetActorForwardVector) (Variables|Default|GetPassVelocity)))
  (Collision|SetCollisionResponsetoChannel (Variables|Default|GetPlayerProjectile) "ECC_GameTraceChannel3" "ECR_Ignore"))

(event Collision|EventHit
  (params (MyComp :type Primitive%20Component%20Object%20Reference) (Other :type Actor%20Object%20Reference) (OtherComp :type Primitive%20Component%20Object%20Reference) (bSelfMoved :type Boolean) (HitLocation :type Vector :default "0, 0, 0") (HitNormal :type Vector :default "0, 0, 0") (NormalImpulse :type Vector :default "0, 0, 0") (Hit :type Hit%20Result%20Structure%20%28by%20ref%29))
  (if (Utilities|DoesObjectImplementInterface Other "/Game/Blueprints/System/BPI_Damageable.BPI_Damageable_C")
    (if (Class|GameplayStatics|ObjectIsA Other "/Game/Blueprints/BP_Player.BP_Player_C")
      _
      (else
        (Class|BPIDamageable|DamageObject(Message) Other (Variables|Default|GetBaseDamage) (Variables|Default|GetBaseWeakPointDamage) (Game|Player|GetPlayerPawn 0) OtherComp)
        (bind _asbp_player (Utilities|Casting|CastToBP_Player (Variables|Actor|GetInstigator))
          (:then
            (Default|HitSuccessFeedback _asbp_player))
          (:CastFailed
            _))
        (Utilities|FlowControl|Delay 0.0))))
  (Actor|DestroyActor))

(fn ConstructionScript)